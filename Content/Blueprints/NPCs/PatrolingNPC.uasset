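; Patrolling stealth-enemy NPC that returns the player to a checkpoint when it keeps them in sight for too long.
; It loops AIMoveTo through patrol points relative to its construction-time transform, waiting between moves.
; AI perception plays an alarm and sets a sight flag, which Tick uses to raise or decay TimeSeen and toggle the Timebar widget.
; The construction script sets visor material and spotlight colour from the Infected flag.
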(event `self.ReceiveBeginPlay`
  (bind _returnvalue (+ (`KismetMathLibrary.GreaterGreater_VectorRotator` (`|GetArrayItem` (`self.Patrol Points`) (`self.PatrolLocation`)) (.rotation (`self.Initial Location`))) (.location (`self.Initial Location`))))
  (bind _astime_bar_ui (cast `/Game/Blueprints/NPCs/TimeBarUI` (`WidgetComponent.GetWidget` (`self.Timebar`))))
  (set `/Game/Blueprints/NPCs/TimeBarUI.ParentInstance` self _astime_bar_ui)
  (if (`AIBlueprintHelperLibrary.IsValidAILocation` _returnvalue)
    (`|AIMoveTo` self _returnvalue null 25.0 :!label _label
      (:`OnSuccess`
        _)
      (:`OnFail`
        _))
    (`GameplayTask_WaitDelay.TaskWaitDelay` (`self.GameplayTasks`) (`self.Wait Time`)
      (:`OnFinish`
        ;[1 1 1] Incriment the counter, and reset to 0 once done.
        (set `self.PatrolLocation` (mod (+ (`self.PatrolLocation`) 1) (`KismetArrayLibrary.Array_Length` (`self.Patrol Points`))))
        (goto _label)))))

(event `self.AIPerception.OnTargetPerceptionUpdated`
  (params (Actor :type "Actor Object Reference") (Stimulus :type "AIStimulus Structure"))
  ;[1 1 1] Update if the player is in the line of sight.
  (cast `/Game/CustomMovement/Blueprints/ExampleCharacter/BP_ExampleCharacter` Actor)
  (bind _output_get (set `self.Player In Sight` (`.bSuccessfullySensed` (break `AIStimulus` Stimulus))))
  (if _output_get
    (`/Engine/EditorBlueprintResources/StandardMacros.DoOnce` false :!label _label_2
      (:`Completed`
        (`GameplayStatics.PlaySoundAtLocation` "/Game/Retro_8Bit_Sounds/Alarms_Sirens/Wavs/AlarmCue.AlarmCue" (`self.K2_GetActorLocation`) (struct) 1.0 1.0 0.0 null null null)
        (`KismetSystemLibrary.Delay` 0.5)
        (goto _label_2 :!via `Reset`)))))

(event `self.ReceiveTick`
  (params (DeltaSeconds :type "Float (single-precision)"))
  (bind _timeseen (`self.TimeSeen`))
  (bind _timebar (`self.Timebar`))
  (if (`self.Player In Sight`)
    (set `self.TimeSeen` (+ DeltaSeconds (`self.TimeSeen`)))
    (if (>= _timeseen 0.0)
      (`SceneComponent.SetVisibility` _timebar true true))
    (if (>= (`self.TimeSeen`) (`self.TimeRequired`))
      (`/Engine/EditorBlueprintResources/StandardMacros.DoOnce` false :!label _label_3
        (:`Completed`
          (`KismetSystemLibrary.PrintString` "Game Over")
          (bind _asbp_example_character (cast `/Game/CustomMovement/Blueprints/ExampleCharacter/BP_ExampleCharacter` (`GameplayStatics.GetPlayerCharacter` 0)))
          (`/Game/CustomMovement/Blueprints/ExampleCharacter/BP_ExampleCharacter.ReturnToCheckpoint` _asbp_example_character)))
      (else
        (goto _label_3 :!via `Reset`)))
    (else
      (set `self.TimeSeen` (`KismetMathLibrary.FMax` (+ (* -1 DeltaSeconds) (`self.TimeSeen`))))
      (if (<= _timeseen 0.0)
        (`SceneComponent.SetVisibility` _timebar false true)))))

(fn `UpdateTimeSeenOnWidget`
  (bind _astime_bar_ui (cast `/Game/Blueprints/NPCs/TimeBarUI` (`WidgetComponent.GetWidget` (`self.Timebar`))))
  (set `/Game/Blueprints/NPCs/TimeBarUI.TimeSeen` (`self.TimeSeen`) _astime_bar_ui))

(fn `UserConstructionScript`
  (set `self.Initial Location` (`self.GetTransform`))
  (if (`self.Infected`)
    (`PrimitiveComponent.SetMaterial` (`self.Mesh`) 1 "/Game/SciFi_Robot/MATERIALS/VISOR/VISOR_MAT.VISOR_MAT")
    (`LightComponent.SetLightColor` (`self.SpotLight`) (struct :`R` 1.0 :`B` 0.404573 :`A` 1.0) true)
    (else
      (`PrimitiveComponent.SetMaterial` (`self.Mesh`) 1 "/Game/SciFi_Robot/MATERIALS/VISOR/VISOR_MAT2_Inst.VISOR_MAT2_Inst")
      (`LightComponent.SetLightColor` (`self.SpotLight`) (struct :`R` 1.0 :`G` 1.0 :`B` 1.0 :`A` 1.0) true))))